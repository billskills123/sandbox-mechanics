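; KeyBP is a key pickup that the player collects by pressing Interact while inside its Box trigger.
; Overlap adds an InteractText widget for any actor, then, for MainThirdPersonCharacter only, enables input and opens a Gate; end overlap removes all widgets and reverses both for the character.
; Interact clears all widgets and, if the Gate is open, sets the character's Key flag and destroys the actor.
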(event `InputAction|Interact`
  (params (Key :type "Key Structure"))
  (:`Pressed`
    (`WidgetLayoutLibrary.RemoveAllWidgets`)
    (`/Engine/EditorBlueprintResources/StandardMacros.Gate` true :!label _label
      (:`Exit`
        (set `/Game/ThirdPersonCPP/Blueprints/MainThirdPersonCharacter.Key` true (stale `self.Box.OnComponentBeginOverlap` _asmain_third_person_character))
        (`self.K2_DestroyActor`)))))

(event `self.Box.OnComponentBeginOverlap`
  (params (OverlappedComponent :type "PrimitiveComponent Object Reference") (OtherActor :type "Actor Object Reference") (OtherComp :type "PrimitiveComponent Object Reference") (OtherBodyIndex :type Integer) (bFromSweep :type Boolean) (SweepResult :type "HitResult Structure (by ref)"))
  (bind _returnvalue (`|CreateWidget` "/Game/Levels/InteractText.InteractText_C"))
  (`UserWidget.AddToViewport` _returnvalue 0)
  (bind _asmain_third_person_character (cast `/Game/ThirdPersonCPP/Blueprints/MainThirdPersonCharacter` OtherActor))
  (`self.EnableInput` (`GameplayStatics.GetPlayerController` 0))
  (goto _label :!via `Open`))

(event `self.Box.OnComponentEndOverlap`
  (params (OverlappedComponent :type "PrimitiveComponent Object Reference") (OtherActor :type "Actor Object Reference") (OtherComp :type "PrimitiveComponent Object Reference") (OtherBodyIndex :type Integer))
  (`WidgetLayoutLibrary.RemoveAllWidgets`)
  (cast `/Game/ThirdPersonCPP/Blueprints/MainThirdPersonCharacter` OtherActor)
  (`self.DisableInput` (`GameplayStatics.GetPlayerController` 0))
  (goto _label :!via `Close`))

(fn `UserConstructionScript`)