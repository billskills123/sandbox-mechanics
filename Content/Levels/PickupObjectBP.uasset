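; Physics sphere pickup object that shows a pickup prompt and can be reset to a spawn position.
; When MainThirdPersonCharacter overlaps the Box, it creates a new PickupText widget and adds it to the viewport, with no removal here.
; It enables player input on BeginPlay, so releasing ResetObject teleports the sphere to ObjectSpawnPosition.
; The reset also zeroes linear velocity and briefly toggles physics simulation off and on.
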(event `self.Box.OnComponentBeginOverlap`
  (params (OverlappedComponent :type "PrimitiveComponent Object Reference") (OtherActor :type "Actor Object Reference") (OtherComp :type "PrimitiveComponent Object Reference") (OtherBodyIndex :type Integer) (bFromSweep :type Boolean) (SweepResult :type "HitResult Structure (by ref)"))
  (cast `/Game/ThirdPersonCPP/Blueprints/MainThirdPersonCharacter` OtherActor)
  (bind _returnvalue (`|CreateWidget` "/Game/Levels/PickupText.PickupText_C"))
  (`UserWidget.AddToViewport` _returnvalue 0))

(event `InputAction|ResetObject`
  (params (Key :type "Key Structure"))
  (bind _sphere (`self.Sphere`))
  (:`Released`
    (`SceneComponent.K2_SetWorldLocation` _sphere (`self.ObjectSpawnPosition`) false true)
    (`PrimitiveComponent.SetSimulatePhysics` _sphere false)
    (`KismetSystemLibrary.Delay` 0.01)
    (`PrimitiveComponent.SetSimulatePhysics` _sphere true)))

(event `InputAction|ResetObject`
  (params (Key :type "Key Structure"))
  (:`Released`
    (`PrimitiveComponent.SetAllPhysicsLinearVelocity` (`self.Sphere`) (0.0 0.0 0.0) false)))

(event `self.ReceiveBeginPlay`
  (`self.EnableInput` (`GameplayStatics.GetPlayerController` 0)))

(fn `UserConstructionScript`)