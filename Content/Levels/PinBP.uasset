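; PinBP is a knockable pin actor that awards the player a point when its Cylinder is displaced.
; It records the Cylinder's start location on BeginPlay and caches the MainThirdPersonCharacter that overlaps its Box.
; Tick checks for movement beyond a small tolerance and, after a one-second Delay, increments that character's Score, updates it through ScoreInterface and destroys the pin.
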(event `self.ReceiveTick`
  (params (DeltaSeconds :type "Float (single-precision)"))
  (bind _maintpc (`self.MainTPC`))
  (bind _maintpc_2 (`self.MainTPC`))
  (bind _output_get (set `self.canAddScore` (!= (`SceneComponent.K2_GetComponentLocation` (`self.Cylinder`)) (`self.StartPosition`) :`ErrorTolerance` 10.0)))
  (`KismetSystemLibrary.Delay` 1.0)
  (if _output_get
    (set `/Game/ThirdPersonCPP/Blueprints/MainThirdPersonCharacter.Score` (+ (`/Game/ThirdPersonCPP/Blueprints/MainThirdPersonCharacter.Score` _maintpc_2) 1) _maintpc_2)
    (`/Game/Levels/ScoreInterface.ChangeScore` (`/Game/ThirdPersonCPP/Blueprints/MainThirdPersonCharacter.ScoreInterface` _maintpc) (`/Game/ThirdPersonCPP/Blueprints/MainThirdPersonCharacter.Score` _maintpc))
    (`self.K2_DestroyActor`)))

(event `self.Box.OnComponentBeginOverlap`
  (params (OverlappedComponent :type "PrimitiveComponent Object Reference") (OtherActor :type "Actor Object Reference") (OtherComp :type "PrimitiveComponent Object Reference") (OtherBodyIndex :type Integer) (bFromSweep :type Boolean) (SweepResult :type "HitResult Structure (by ref)"))
  (bind _asmain_third_person_character (cast `/Game/ThirdPersonCPP/Blueprints/MainThirdPersonCharacter` OtherActor))
  (set `self.MainTPC` _asmain_third_person_character))

(event `self.ReceiveBeginPlay`
  (set `self.StartPosition` (`SceneComponent.K2_GetComponentLocation` (`self.Cylinder`))))

(fn `UserConstructionScript`)