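; Interactable locked door that swings open or closed on Interact, provided the player's MainThirdPersonCharacter has its Key.
; A box overlap shows an interact prompt, enables input and opens a Gate; leaving clears all widgets, disables input and closes the Gate.
; With the key, a FlipFlop plays or reverses a timeline that lerps the door's yaw between closed and open angles; without it, a locked message appears.
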(event `InputAction|Interact`
  (params (Key :type "Key Structure"))
  (:`Pressed`
    (if (`/Game/ThirdPersonCPP/Blueprints/MainThirdPersonCharacter.Key` (stale `self.Box.OnComponentBeginOverlap` _asmain_third_person_character))
      (`/Engine/EditorBlueprintResources/StandardMacros.Gate` true :!label _label
        (:`Exit`
          (`/Engine/EditorBlueprintResources/StandardMacros.FlipFlop`
            (:`A`
              (bind (_direction _doormovement) (`Timeline|DoorMovement` :!label _label_2)
                (:`Update`
                  (`SceneComponent.K2_SetRelativeRotation` (`self.Door`) (`KismetMathLibrary.MakeRotator` 0.0 0.0 (`KismetMathLibrary.Lerp` (`self.ClosedAngle`) (`self.OpenAngle`) _doormovement)) false false))))
            (:`B`
              (goto _label_2 :!via `Reverse`)))))
      (else
        (`WidgetLayoutLibrary.RemoveAllWidgets`)
        (bind _returnvalue (`|CreateWidget` "/Game/Levels/LockedText.LockedText_C"))
        (`UserWidget.AddToViewport` _returnvalue 0)))))

(event `self.Box.OnComponentBeginOverlap`
  (params (OverlappedComponent :type "PrimitiveComponent Object Reference") (OtherActor :type "Actor Object Reference") (OtherComp :type "PrimitiveComponent Object Reference") (OtherBodyIndex :type Integer) (bFromSweep :type Boolean) (SweepResult :type "HitResult Structure (by ref)"))
  (bind _returnvalue (`|CreateWidget` "/Game/Levels/InteractText.InteractText_C"))
  (`UserWidget.AddToViewport` _returnvalue 0)
  (bind _asmain_third_person_character (cast `/Game/ThirdPersonCPP/Blueprints/MainThirdPersonCharacter` OtherActor))
  (`self.EnableInput` (`GameplayStatics.GetPlayerController` 0))
  (goto _label :!via `Open`))

(event `self.Box.OnComponentEndOverlap`
  (params (OverlappedComponent :type "PrimitiveComponent Object Reference") (OtherActor :type "Actor Object Reference") (OtherComp :type "PrimitiveComponent Object Reference") (OtherBodyIndex :type Integer))
  (`WidgetLayoutLibrary.RemoveAllWidgets`)
  (cast `/Game/ThirdPersonCPP/Blueprints/MainThirdPersonCharacter` OtherActor)
  (`self.DisableInput` (`GameplayStatics.GetPlayerController` 0))
  (goto _label :!via `Close`))

(fn `UserConstructionScript`)