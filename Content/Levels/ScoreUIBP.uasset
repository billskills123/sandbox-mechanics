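; ScoreUIBP is a trigger volume that controls the score UI for the MainThirdPersonCharacter.
; On entering the box, it creates a ScoreInterface widget, stores it on the character, adds it to the viewport and passes in the current score.
; On leaving, it resets the character's Score to zero and calls RemoveAllWidgets, which clears every widget from the viewport, not just the score display.
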(event `self.Box.OnComponentBeginOverlap`
  (params (OverlappedComponent :type "PrimitiveComponent Object Reference") (OtherActor :type "Actor Object Reference") (OtherComp :type "PrimitiveComponent Object Reference") (OtherBodyIndex :type Integer) (bFromSweep :type Boolean) (SweepResult :type "HitResult Structure (by ref)"))
  (bind _asmain_third_person_character (cast `/Game/ThirdPersonCPP/Blueprints/MainThirdPersonCharacter` OtherActor))
  (bind _returnvalue (`|CreateWidget` "/Game/Levels/ScoreInterface.ScoreInterface_C"))
  (bind _output_get (set `/Game/ThirdPersonCPP/Blueprints/MainThirdPersonCharacter.ScoreInterface` _returnvalue _asmain_third_person_character))
  (`UserWidget.AddToViewport` _output_get 0)
  (bind _output_get_2 (set `self.ScoreInterface` _output_get))
  (`/Game/Levels/ScoreInterface.ChangeScore` _output_get_2 (`/Game/ThirdPersonCPP/Blueprints/MainThirdPersonCharacter.Score` _asmain_third_person_character)))

(event `self.Box.OnComponentEndOverlap`
  (params (OverlappedComponent :type "PrimitiveComponent Object Reference") (OtherActor :type "Actor Object Reference") (OtherComp :type "PrimitiveComponent Object Reference") (OtherBodyIndex :type Integer))
  (bind _asmain_third_person_character (cast `/Game/ThirdPersonCPP/Blueprints/MainThirdPersonCharacter` OtherActor))
  (`WidgetLayoutLibrary.RemoveAllWidgets`)
  (set `/Game/ThirdPersonCPP/Blueprints/MainThirdPersonCharacter.Score` 0 _asmain_third_person_character))

(fn `UserConstructionScript`)